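; Player Blueprint (BP_TDPlayer) that sets up a fixed view angle and the main HUD, with debug-style keys for changing the view.
; On BeginPlay it sets the actor to a hard-coded rotation, then creates W_MainHUD and adds it to the viewport.
; FlipFlops on raw key presses toggle the camera between perspective and orthographic projection (C) and remove or re-add the HUD (W).
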(event EventBeginPlay
  (|CallParentFunction)
  (Transformation|SetActorRotation "-20.000000,-90.000000,0.000000")
  (bind _returnvalue (UserInterface|CreateWidget "/Game/Blueprint/UI/W_MainHUD.W_MainHUD_C"))
  (bind _output_get (Variables|Default|SetMain_HUD _returnvalue))
  (UserInterface|Viewport|AddtoViewport _output_get 0))

(event Input|KeyboardEvents|C
  (params (Key :type Key%20Structure))
  (bind _camera (Variables|Default|GetCamera))
  (:Pressed
    (Utilities|FlowControl|FlipFlop
      (:A
        (Class|CameraComponent|SetProjectionMode _camera "Perspective"))
      (:B
        (Class|CameraComponent|SetProjectionMode _camera "Orthographic")))))

(event Input|KeyboardEvents|W
  (params (Key :type Key%20Structure))
  (bind _main_hud (Variables|Default|GetMain_HUD))
  (:Pressed
    (Utilities|FlowControl|FlipFlop
      (:A
        (Widget|RemovefromParent _main_hud))
      (:B
        (UserInterface|Viewport|AddtoViewport _main_hud 0)))))

(fn ConstructionScript)