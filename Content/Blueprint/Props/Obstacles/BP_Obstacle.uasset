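; BP_Obstacle is a clickable obstacle prop that offers the player a paid destruction option through a widget.
; On BeginPlay it passes its name and destruction cost to the W_DestroyObstacle widget in its WidgetComponent, binds an event to the widget's destroy action, then hides it.
; Clicking the mesh component makes the widget visible.
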(event OnClicked(MeshComponent)
  (params (TouchedComponent :type Primitive%20Component%20Object%20Reference) (ButtonPressed :type Key%20Structure))
  (Widget|SetVisibility (Variables|Default|GetWidget) "Visible"))

(event EventBeginPlay
  (bind _output_get (Variables|Default|SetWidget (.AsW%20Destroy%20Obstacle (Utilities|Casting|CastToW_DestroyObstacle (UserInterface|GetWidget (Variables|Default|GetWidgetComponent))))))
  (Default|SetObstacleName _output_get (Variables|Default|GetObstacleName))
  (Default|SetObstacleDestructionCost _output_get (Variables|Default|GetObstacleDestructionCost))
  (EventDispatchers|BindEventtoDestroyObstacle _output_get (EventDispatchers|CreateEvent :!event DestroyObstacle))
  (Widget|SetVisibility _output_get "Hidden"))

(fn ConstructionScript)