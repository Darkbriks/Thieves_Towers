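; BP_TDPlayer is a player Blueprint for the Thieves Towers game that currently has no active logic of its own.
; BeginPlay and the construction script are empty.
; A disconnected test chain, which never runs, repeatedly waits on a Delay, casts the game instance to GA_ThievesTowers and calls AddCardToHand with BP_TestCard to fill the hand one card at a time.
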(event EventBeginPlay)

(fn ConstructionScript)